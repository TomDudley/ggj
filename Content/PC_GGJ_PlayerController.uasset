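; Player controller that moves its controlled pawn to a floor tile clicked with the left mouse button.
; Each click deprojects the cursor and runs a persistently debug-drawn Visibility line trace, whose end point multiplies world location by normalized direction instead of offsetting along it.
; If the hit actor's class is exactly FloorTile, the pawn is set to that tile's location with a sweep and no teleport.
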(event Input|MouseEvents|LeftMouseButton
  (params (Key :type Key%20Structure :default "AnyKey"))
  (bind (_worldlocation _worlddirection) (Game|Player|ConvertMouseLocationToWorldSpace))
  (:Pressed
    (bind _outhit (Collision|LineTraceByChannel _worldlocation (* _worldlocation (Math|Vector|Normalize _worlddirection)) "TraceTypeQuery1" false 0 "Persistent"))
    (if (== (Utilities|GetClass (.HitActor (Collision|BreakHitResult _outhit))) "/Game/floorTile.floorTile_C")
      (Transformation|SetActorLocation (Pawn|GetControlledPawn) (Transformation|GetActorLocation (.HitActor (Collision|BreakHitResult _outhit))) true false))))

(fn ConstructionScript)